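; BP_Enemy is an obstacle enemy that damages BP_Player on contact and destroys itself once it falls behind the player on the X axis.
; Tick looks up the player and compares X locations.
; Box overlap either consumes the player's shield, leaving the enemy alive, or deducts health, updates the health bar and destroys the enemy.
; A lethal hit also flags death and displays restart.
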(event `self.ReceiveTick`
  (params (DeltaSeconds :type "Float (single-precision)"))
  (bind _returnvalue (`GameplayStatics.GetActorOfClass` "/Game/InfiniteMatrix/Blueprints/BP_Player.BP_Player_C"))
  (if (< (.x (.location (`self.GetTransform`))) (.x (.location (`self.GetTransform` _returnvalue))))
    (`self.K2_DestroyActor`)))

(event `self.Box.OnComponentBeginOverlap`
  (params (OverlappedComponent :type "PrimitiveComponent Object Reference") (OtherActor :type "Actor Object Reference") (OtherComp :type "PrimitiveComponent Object Reference") (OtherBodyIndex :type Integer) (bFromSweep :type Boolean) (SweepResult :type "HitResult Structure (by ref)"))
  (bind _asbp_player (cast `/Game/InfiniteMatrix/Blueprints/BP_Player` OtherActor))
  (if (`/Game/InfiniteMatrix/Blueprints/BP_Player.Shielded` _asbp_player)
    (set `/Game/InfiniteMatrix/Blueprints/BP_Player.Shielded` false _asbp_player)
    (`Widget.RemoveFromParent` (`/Game/InfiniteMatrix/Blueprints/BP_Player.WB Shield` _asbp_player))
    (else
      (bind _health (`/Game/InfiniteMatrix/Blueprints/BP_Player.Health` _asbp_player))
      (if (<= _health 25.0)
        (bind _output_get (set `/Game/InfiniteMatrix/Blueprints/BP_Player.Health` 0.0 _asbp_player))
        (bind _wb_healthbar (`/Game/InfiniteMatrix/Blueprints/BP_Player.WB_HealthBar` _asbp_player))
        (`/Game/InfiniteMatrix/Blueprints/WB_HealthBar.UpdateHealthBar` _wb_healthbar _output_get)
        (set `/Game/InfiniteMatrix/Blueprints/BP_Player.IsDead` true _asbp_player)
        (`/Game/InfiniteMatrix/Blueprints/BP_Player.DisplayRestart` _asbp_player)
        (else
          (bind _output_get_2 (set `/Game/InfiniteMatrix/Blueprints/BP_Player.Health` (- _health 25.0) _asbp_player))
          (`/Game/InfiniteMatrix/Blueprints/WB_HealthBar.UpdateHealthBar` _wb_healthbar _output_get_2)))
      (`self.K2_DestroyActor`))))

(fn `UserConstructionScript`)